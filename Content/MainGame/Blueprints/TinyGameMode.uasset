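; TinyGameMode is a game mode Blueprint that owns the pause menu and toggles the game's paused state.
; CreatePauseMenu builds a hidden BPW_PauseMenuWrapper widget on the viewport.
; PauseGame toggles it, switching input mode and notifying the menu, and fakes pausing with near-zero global time dilation rather than a true pause.
; UnPauseGame and BeginPlay are empty, and nothing in this file calls either working function.
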(event `self.ReceiveBeginPlay`)

(fn `CreatePauseMenu`
  (bind _returnvalue (`|CreateWidget` "/Game/MainGame/UI/BPW_PauseMenuWrapper.BPW_PauseMenuWrapper_C" (`GameplayStatics.GetPlayerController` 0)))
  (bind _output_get (set `self.PauseMenu` _returnvalue))
  (`Widget.SetVisibility` _output_get "Hidden")
  (`UserWidget.AddToViewport` (`self.PauseMenu`) 0))

(fn `PauseGame`
  ;[1 1 1] Handles pausing and unpausing the game - showing pause menu
  (if (`self.GameIsPaused`)
    (set `self.GameIsPaused` false)
    (`GameplayStatics.SetGlobalTimeDilation` 1.0)
    (`Widget.SetVisibility` (`self.PauseMenu`) "Hidden")
    (`WidgetBlueprintLibrary.SetInputMode_GameOnly` (`GameplayStatics.GetPlayerController` 0))
    (`/Game/MainGame/UI/BPW_PauseMenuWrapper.OnHide` (`self.PauseMenu`))
    (else
      (set `self.GameIsPaused` true)
      (`GameplayStatics.SetGlobalTimeDilation` 0.0001)
      (`Widget.SetVisibility` (`self.PauseMenu`) "Visible")
      (`WidgetBlueprintLibrary.SetInputMode_GameAndUIEx` (`GameplayStatics.GetPlayerController` 0) (`PanelWidget.GetChildAt` (`/Game/MainGame/UI/BPW_PauseMenuWrapper.WidgetSwitcher_0` (`self.PauseMenu`)) 0))
      (`/Game/MainGame/UI/BPW_PauseMenuWrapper.OnShow` (`self.PauseMenu`)))))

(fn `UnPauseGame`)

(fn `UserConstructionScript`)