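; BP_WorldActor is an item placed in the world that adds itself to an inventory when overlapped.
; On BeginPlay it looks up its ID in DT_Items and copies the name and world mesh, raising Amount to the table value if that is higher.
; Its sphere collider's overlap casts the other actor to TinyPlayerController and passes itself to that InventoryComponent's AddItemToInventory.
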(event `self.ReceiveBeginPlay`
  (`parent.ReceiveBeginPlay`)
  (`self.LoadInventoryItem`))

(event `self.SphereCollider.OnComponentBeginOverlap`
  (params (OverlappedComponent :type "PrimitiveComponent Object Reference") (OtherActor :type "Actor Object Reference") (OtherComp :type "PrimitiveComponent Object Reference") (OtherBodyIndex :type Integer) (bFromSweep :type Boolean) (SweepResult :type "HitResult Structure (by ref)"))
  (bind _astiny_player_controller (cast `/Game/MainGame/Character/TinyPlayerController` OtherActor))
  (`/Game/MainGame/Inventory/Components/InventoryComponent.AddItemToInventory` (`/Game/MainGame/Character/TinyPlayerController.InventoryComponent` _astiny_player_controller) self))

(fn `LoadInventoryItem`
  (returns (Success :type Boolean))
  (bind _returnvalue (`|GetDataTableRow` "/Game/MainGame/Items/DT_Items.DT_Items" (`self.ID`))
    (:`then`
      (bind _output_get (set `self.InventoryItem` _returnvalue))
      (bind (_id _icon _name _description _itemtype _itemcategory _amount _isstackable _maxstacksize _isdroppable _worldmesh) (break `/Game/MainGame/Inventory/Struct_InventoryItem` _output_get))
      (set `self.Name` _name)
      (if (> _amount (`self.Amount`))
        (set `self.Amount` _amount))
      (if (`KismetSystemLibrary.IsValid` _worldmesh)
        (set `self.WorldMesh` _worldmesh))
      (return true))))

(fn `UserConstructionScript`
  (`parent.UserConstructionScript`))