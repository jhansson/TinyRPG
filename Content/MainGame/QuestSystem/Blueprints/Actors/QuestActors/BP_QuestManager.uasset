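; Quest manager actor that registers quests and tracks which one is currently selected.
; AddNewQuest rejects invalid or already added classes, spawns a quest actor, sets up its starting goal and links it to a new entry in the main widget's quest list.
; It auto-selects the quest if requested or if it is the first.
; SelectedNewQuest updates the previous and new quest widgets; the OnSwitchSubQuest event is empty.
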(event `self.ReceiveBeginPlay`)

(event `OnSwitchSubQuest`)

(fn `AddNewQuest`
  (params (QuestClass :type "/Game/MainGame/QuestSystem/Blueprints/Actors/QuestActors/BP_MasterQuest Class Reference") (`DireclyStart?` :type Boolean))
  (returns (Success :type Boolean))
  (locals (`Start?` :type Boolean) (localClass :type "/Game/MainGame/QuestSystem/Blueprints/Actors/QuestActors/BP_MasterQuest Class Reference") (LocalQuestActor :type "/Game/MainGame/QuestSystem/Blueprints/Actors/QuestActors/BP_MasterQuest Object Reference"))
  (bind _localquestactor (`local.LocalQuestActor`))
  (set `local.localClass` QuestClass)
  (set `local.Start?` `DireclyStart?`)
  (if (and (`KismetSystemLibrary.IsValidClass` QuestClass) (not (`KismetArrayLibrary.Array_Contains` (`self.AllQuestClasses`) QuestClass)))
    (`KismetArrayLibrary.Array_Add` (`self.AllQuestClasses`) (`local.localClass`))
    (bind _returnvalue (`|SpawnActorFromClass` :`Class` (`local.localClass`) :`SpawnTransform` (`KismetMathLibrary.MakeTransform` (0.0 0.0 0.0)) :`CollisionHandlingOverride` "AlwaysSpawn" :`TransformScaleMethod` "OverrideRootScale" :`QuestWIdget` null :`Instigator` null))
    (bind _output_get (set `local.LocalQuestActor` _returnvalue))
    (`KismetArrayLibrary.Array_Add` (`self.QuestActors`) _output_get)
    (`/Game/MainGame/QuestSystem/Blueprints/Actors/QuestActors/BP_MasterQuest.SetupStartingGoal` _localquestactor)
    (bind _widget (`/Game/MainGame/QuestSystem/Widgets/MainWidget.AddQuestToList` (`self.MainWidget`) _localquestactor))
    (bind _output_get_2 (set `/Game/MainGame/QuestSystem/Blueprints/Actors/QuestActors/BP_MasterQuest.QuestWIdget` _widget (`local.LocalQuestActor`)))
    (`/Game/MainGame/QuestSystem/Widgets/QuestWidget.UpdateQuest` _output_get_2)
    (if (or (`local.Start?`) (<= (`KismetArrayLibrary.Array_Length` (`self.QuestActors`)) 1))
      (`self.SelectedNewQuest` (`local.LocalQuestActor`) (`|GetArrayItem` (`/Game/MainGame/QuestSystem/Widgets/QuestWidget.SubGoalWidets` (`/Game/MainGame/QuestSystem/Blueprints/Actors/QuestActors/BP_MasterQuest.QuestWIdget` (`local.LocalQuestActor`))))))
    (return true)
    (else
      (return false))))

(fn `SelectedNewQuest`
  (params (Quest :type "/Game/MainGame/QuestSystem/Blueprints/Actors/QuestActors/BP_MasterQuest Object Reference") (SubGoal :type "/Game/MainGame/QuestSystem/Widgets/SubGoalWidget Object Reference"))
  (bind _currentquest (`self.CurrentQuest`))
  (bind _questwidget (`/Game/MainGame/QuestSystem/Blueprints/Actors/QuestActors/BP_MasterQuest.QuestWIdget` _currentquest))
  (`/Engine/EditorBlueprintResources/StandardMacros.IsValid` _currentquest
    (:`Is Valid`
      (`Widget.SetIsEnabled` (`/Game/MainGame/QuestSystem/Widgets/QuestWidget.QuestName` _questwidget) false)
      (`/Game/MainGame/QuestSystem/Widgets/QuestWidget.SelectSubGoal` _questwidget null))
    (:`Is Not Valid`
      _))
  (bind _output_get (set `self.CurrentQuest` Quest))
  (`/Game/MainGame/QuestSystem/Widgets/QuestWidget.OnQuestSelected` (`/Game/MainGame/QuestSystem/Blueprints/Actors/QuestActors/BP_MasterQuest.QuestWIdget` _output_get) SubGoal)
  (return))

(fn `UserConstructionScript`)