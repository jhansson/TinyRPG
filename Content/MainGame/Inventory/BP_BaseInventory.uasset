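; Base inventory that stores picked-up items in per-category slot lists such as weapons, armor, food and key items.
; AddItemToInventory merges stackables into a non-full slot with the same ID, otherwise adds a slot if space allows, then destroys the item actor.
; Merging adds the whole amount without clamping to max stack size.
; Weight checks are placeholders: current weight is always 1, and HasEnoughWeightLeft always returns false.
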(fn `AddItemToInventory`
  (params (InActor :type "/Game/MainGame/Inventory/Usables/BP_WorldActor Object Reference"))
  (returns (Index :type Integer))
  (locals (LocalItem :type "/Game/MainGame/Inventory/Usables/BP_WorldActor Object Reference"))
  (bind _output_get (set `local.LocalItem` InActor))
  (bind (_inventoryitem_id _inventoryitem_icon _inventoryitem_name _inventoryitem_description _inventoryitem_itemtype _inventoryitem_itemcategory _inventoryitem_amount _inventoryitem_isstackable) (break `/Game/MainGame/Inventory/Struct_InventoryItem` (`/Game/MainGame/Inventory/Usables/BP_WorldActor.InventoryItem` _output_get)))
  (if _inventoryitem_isstackable
    (bind (_addedtostack _index) (`self.TryToAddToPartialStack` (`local.LocalItem`)))
    (if _addedtostack
      (bind _output_get_2 (set `self.IndexAdded` _index))
      (`self.K2_DestroyActor` (`local.LocalItem`) :!label _label)
      (return _output_get_2)
      (else
        (bind _hasspace (`self.HasInventorySpace` :!label _label_2)
          (:`Out`
            (if _hasspace
              (bind _returnvalue (`KismetArrayLibrary.Array_Add` (select `/Game/MainGame/Inventory/Enum_ItemCategory` _inventoryitem_itemcategory :`NewEnumerator0` (`self.WeaponList`) :`NewEnumerator1` (`self.BowArrowList`) :`NewEnumerator4` (`self.ShieldList`) :`NewEnumerator2` (`self.ArmorList`) :`NewEnumerator3` (`self.MaterialList`) :`NewEnumerator5` (`self.FoodList`) :`NewEnumerator6` (`self.KeyItemList`)) (make `/Game/MainGame/Inventory/InventorySlot` (`/Game/MainGame/Inventory/Usables/BP_WorldActor.InventoryItem` (`local.LocalItem`)) _inventoryitem_amount)))
              (set `self.IndexAdded` _returnvalue)
              (goto _label))))))
    (else
      (goto _label_2))))

(fn `CanItemStack`
  (params (Item :type "/Game/MainGame/Inventory/BP_BaseItem Object Reference"))
  (returns (Stackable :type Boolean))
  (return (`/Game/MainGame/Inventory/BP_BaseItem.IsStackable` Item)))

(fn `GetCurrentWeight`
  (returns (Weight :type Integer))
  (return 1))

(fn `HasEnoughWeightLeft`
  (params (Item :type "/Game/MainGame/Inventory/BP_BaseItem Object Reference"))
  (returns (EnoughWeight :type Boolean))
  (return false))

(fn `TryToAddToPartialStack`
  (params (Item :type "/Game/MainGame/Inventory/Usables/BP_WorldActor Object Reference"))
  (returns (AddedToStack :type Boolean) (Index :type Integer))
  (locals (LocalInventory :type "/Game/MainGame/Inventory/InventorySlot Structure") (PartialIndex :type Integer) (HasPartial :type Boolean) (LocalItem :type "/Game/MainGame/Inventory/Usables/BP_WorldActor Object Reference") (LocalItemCategory :type "/Game/MainGame/Inventory/Enum_ItemCategory Enum"))
  (bind _returnvalue (select `/Game/MainGame/Inventory/Enum_ItemCategory` (`local.LocalItemCategory`) :`NewEnumerator0` (`self.WeaponList`) :`NewEnumerator1` (`self.BowArrowList`) :`NewEnumerator4` (`self.ShieldList`) :`NewEnumerator2` (`self.ArmorList`) :`NewEnumerator3` (`self.MaterialList`) :`NewEnumerator5` (`self.FoodList`) :`NewEnumerator6` (`self.KeyItemList`)))
  (bind (_item _slotcount) (break `/Game/MainGame/Inventory/InventorySlot` (`|GetArrayItem` _returnvalue (`local.PartialIndex`))))
  (bind _output_get (set `local.LocalItem` Item)) ; Save for easier access
  (bind (_id _icon _name _description _itemtype _itemcategory) (break `/Game/MainGame/Inventory/Struct_InventoryItem` (`/Game/MainGame/Inventory/Usables/BP_WorldActor.InventoryItem` _output_get)))
  (set `local.LocalItemCategory` _itemcategory)
  (for (_array_element _array_index) (select `/Game/MainGame/Inventory/Enum_ItemCategory` _itemcategory :`NewEnumerator0` (`self.WeaponList`) :`NewEnumerator1` (`self.BowArrowList`) :`NewEnumerator4` (`self.ShieldList`) :`NewEnumerator2` (`self.ArmorList`) :`NewEnumerator3` (`self.MaterialList`) :`NewEnumerator5` (`self.FoodList`) :`NewEnumerator6` (`self.KeyItemList`))
    (set `local.PartialIndex` _array_index)
    (bind (_item_2 _slotcount_2) (break `/Game/MainGame/Inventory/InventorySlot` _array_element))
    (bind (_id_2 _icon_2 _name_2 _description_2 _itemtype_2 _itemcategory_2 _amount _isstackable _maxstacksize) (break `/Game/MainGame/Inventory/Struct_InventoryItem` _item_2))
    (bind _output_get_2 (set `local.HasPartial` (and (== _id_2 (`/Game/MainGame/Inventory/Usables/BP_WorldActor.ID` (`local.LocalItem`))) (< _slotcount_2 _maxstacksize)))) ; Set to partial if correct name and stack isn't full
    (if _output_get_2
      (break)))
  (if (`local.HasPartial`)
    (bind _structout (setmembers `/Game/MainGame/Inventory/InventorySlot` :`StructRef` (make `/Game/MainGame/Inventory/InventorySlot` _item (+ _slotcount (`.Amount_14_EC0B2777411E3E114BCA68AE41761B73` (break `/Game/MainGame/Inventory/Struct_InventoryItem` (`/Game/MainGame/Inventory/Usables/BP_WorldActor.InventoryItem` (`local.LocalItem`))))))))
    (`KismetArrayLibrary.Array_Set` _returnvalue (`local.PartialIndex`) _structout true))
  (return (`local.HasPartial`) (`local.PartialIndex`)))

(fn `UserConstructionScript`)