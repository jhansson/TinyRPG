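; Character preview actor for the inventory that shows equipped items on a separate model through a scene capture.
; The capture renders only this actor, and Tick sets its custom time dilation to the inverse of global dilation so it runs at normal speed.
; EquipItem and UnEquipItem set or clear the slot's skeletal mesh, linking head, body and legs to the main mesh's pose, while hand slots stay independent.
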(event `self.ReceiveBeginPlay`
  (set `SceneCaptureComponent.ShowOnlyActors` (`|MakeArray` self :!type "Actor Object Reference") (`self.SceneCaptureComponent2D`)))

(event `self.ReceiveTick`
  (params (DeltaSeconds :type "Float (single-precision)"))
  (set `self.CustomTimeDilation` (/ 1.0 (`GameplayStatics.GetGlobalTimeDilation`))))

(fn `EquipItem`
  (params (Item :type "/Game/MainGame/Inventory/Struct_InventoryItem Structure"))
  (bind ((`EquipmentMesh_51_6734145F4963CAEE2AED39849D8F6D50` _equipmentmesh) (`EquipmentSlot_57_51932A264CF1B23B08E3D5BB7F01E715` _equipmentslot)) (break `/Game/MainGame/Inventory/Struct_InventoryItem` Item))
  (bind _returnvalue (select `/Game/MainGame/Inventory/Enum_EquipmentSlots` _equipmentslot :`NewEnumerator0` (`self.Head`) :`NewEnumerator1` (`self.Body`) :`NewEnumerator4` (`self.Legs`) :`NewEnumerator11` (`self.MainHand`) :`NewEnumerator12` (`self.OffHand`) :!type "SkinnedMeshComponent Object Reference"))
  (`SkinnedMeshComponent.SetSkinnedAssetAndUpdate` _returnvalue _equipmentmesh true)
  (if (not (or (== _returnvalue (`self.MainHand`)) (== _returnvalue (`self.OffHand`))))
    (`SkinnedMeshComponent.SetLeaderPoseComponent` _returnvalue (`self.SkeletalMesh`))))

(fn `UnEquipItem`
  (params (Item :type "/Game/MainGame/Inventory/Struct_InventoryItem Structure"))
  (bind _returnvalue (select `/Game/MainGame/Inventory/Enum_EquipmentSlots` (`.EquipmentSlot_57_51932A264CF1B23B08E3D5BB7F01E715` (break `/Game/MainGame/Inventory/Struct_InventoryItem` Item)) :`NewEnumerator0` (`self.Head`) :`NewEnumerator1` (`self.Body`) :`NewEnumerator4` (`self.Legs`) :`NewEnumerator11` (`self.MainHand`) :`NewEnumerator12` (`self.OffHand`) :!type "SkinnedMeshComponent Object Reference"))
  (`SkinnedMeshComponent.SetSkinnedAssetAndUpdate` _returnvalue null true)
  (if (not (or (== _returnvalue (`self.MainHand`)) (== _returnvalue (`self.OffHand`))))
    (`SkinnedMeshComponent.SetLeaderPoseComponent` _returnvalue (`self.SkeletalMesh`))))

(fn `UserConstructionScript`)