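; Base usable world actor that represents an inventory item placed in the level.
; LoadInventoryItem looks up its ID in a data table chosen by item type, with tables set only for consumables and equipment.
; A found row fills the item struct, name and, if valid, the world mesh variable, while a missing row prints a not-found message.
; The event graph holds only disabled default events.
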(fn `LoadInventoryItem`
  (returns (Success :type Boolean))
  ;[1 1 1] Load data from datatable
  (bind _returnvalue (`|GetDataTableRow` (select `/Game/Playground/Jimmy/Inventory/Jimmy_Enum_ItemType` (`self.ItemType`) :`NewEnumerator1` (`self.ConsumablesDataTable`) :`NewEnumerator0` (`self.EquipmentDataTable`)) (`self.ID`))
    (:`then`
      (bind _output_get (set `self.InventoryItem` _returnvalue))
      (bind (_id _icon _name _description _quality _itemtype _amount _isstackable _maxstacksize _isdroppable _worldmesh) (break `/Game/Playground/Jimmy/Inventory/Jimmy_Struct_InventoryItem` _output_get))
      (set `self.Name` _name)
      (if (`KismetSystemLibrary.IsValid` _worldmesh)
        (set `self.WorldMesh` _worldmesh))
      (return true))
    (:`RowNotFound`
      (`KismetSystemLibrary.PrintString` (`KismetStringLibrary.BuildString_Name` "" " NOT FOUND" (`self.ID`))))))

(fn `UserConstructionScript`
  (`parent.UserConstructionScript`))