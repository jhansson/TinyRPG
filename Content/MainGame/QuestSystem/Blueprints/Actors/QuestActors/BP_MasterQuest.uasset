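; BP_MasterQuest is a quest actor that tracks which sub-goals of its quest are currently active.
; SetupStartingGoal copies the starting indices into the current indices, and UpdateSubGoals rebuilds the current goal list from QuestInfo's SubGoals.
; GoToNextSubGoal replaces all active indices with the one after the highest, returning false when no further sub-goal exists.
; Its event graph holds only disabled stubs, so these functions run only when called.
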(fn `GoToNextSubGoal`
  (returns (Success :type Boolean))
  (locals (NextIndex :type Integer :default 0))
  (bind _currentgoalindices (`self.CurrentGoalIndices`))
  (bind _returnvalue (+ (`.MaxValue` (`KismetMathLibrary.MaxOfIntArray` (`self.CurrentGoalIndices`))) 1))
  (if (<= _returnvalue (`KismetArrayLibrary.Array_LastIndex` (`.SubGoals_24_8D71AFD043B0AF618D06F2A24AC2BF1D` (break `/Game/MainGame/QuestSystem/Blueprints/Structures/S_QuestInfo` (`self.QuestInfo`)))))
    (set `local.NextIndex` _returnvalue)
    (`KismetArrayLibrary.Array_Clear` _currentgoalindices)
    (`KismetArrayLibrary.Array_Add` _currentgoalindices (`local.NextIndex`))
    (`self.UpdateSubGoals`)
    (return true)
    (else
      (return false))))

(fn `SetupStartingGoal`
  (`KismetArrayLibrary.Array_Clear` (`self.CurrentGoalIndices`))
  (set `self.CurrentGoalIndices` (`self.StartingSubGoalIndices`))
  (`self.UpdateSubGoals`)
  (return))

(fn `UpdateSubGoals`
  (`KismetArrayLibrary.Array_Clear` (`self.CurrentGoals`))
  (for _array_element (`self.CurrentGoalIndices`)
    (`KismetArrayLibrary.Array_Add` (`self.CurrentGoals`) (`|GetArrayItem` (`.SubGoals_24_8D71AFD043B0AF618D06F2A24AC2BF1D` (break `/Game/MainGame/QuestSystem/Blueprints/Structures/S_QuestInfo` (`self.QuestInfo`))) _array_element)))
  (return))

(fn `UserConstructionScript`)